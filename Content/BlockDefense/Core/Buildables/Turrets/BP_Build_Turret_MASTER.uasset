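; Master Blueprint for buildable turrets in Block Defense, handling creation visuals and selection highlighting, with no attack logic in these graphs.
; The construction script creates dynamic materials for the cannon and base, whose IsHighlighted parameter is toggled by the selection events.
; On BeginPlay a timeline drives the Niagara Progress and Opacity variables for a growth effect.
; OnHit is a stub, beam-spawning nodes are unconnected, and deselection prints a debug string.
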(event `self.ReceiveBeginPlay`
  (bind _niagara (`self.Niagara`))
  (bind (_direction _towergrowth _opacity) (`Timeline|Timeline_Creation`)
    (:`Update`
      (`NiagaraComponent.SetVariableFloat` _niagara "Progress" _towergrowth)
      (`NiagaraComponent.SetVariableFloat` _niagara "Opacity" _opacity))))

(event `self.OnHit`
  (params (HitUnit :type "EnemyBase Object Reference"))
  (`/Engine/EditorBlueprintResources/StandardMacros.IsValid` HitUnit))

(event `self.OnSelectEnd`
  (`KismetSystemLibrary.PrintString` "Hello")
  (`MaterialInstanceDynamic.SetScalarParameterValue` (`self.Cannon_MI`) "IsHighlighted" 0.0)
  (`MaterialInstanceDynamic.SetScalarParameterValue` (`self.Base_MI`) "IsHighlighted" 0.0))

(event `self.OnSelectStart`
  (`MaterialInstanceDynamic.SetScalarParameterValue` (`self.Cannon_MI`) "IsHighlighted" 1.0)
  (`MaterialInstanceDynamic.SetScalarParameterValue` (`self.Base_MI`) "IsHighlighted" 1.0))

(fn `UserConstructionScript`
  (bind _returnvalue (`PrimitiveComponent.CreateDynamicMaterialInstance` (`self.Cannon`) 0 (`self.CannonClass`) "None"))
  (set `self.Cannon_MI` _returnvalue)
  (bind _returnvalue_2 (`PrimitiveComponent.CreateDynamicMaterialInstance` (`self.Base`) 0 (`self.BaseClass`) "None"))
  (set `self.Base_MI` _returnvalue_2))