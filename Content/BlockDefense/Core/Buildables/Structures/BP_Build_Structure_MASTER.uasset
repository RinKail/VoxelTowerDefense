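; Master Blueprint for a Block Defense buildable structure, handling its build effect, idle spin and selection highlight.
; On BeginPlay, a timeline feeds growth and opacity curves into Niagara, while Tick continuously yaws the Scene component.
; The construction script creates dynamic materials for the structure and type meshes.
; Selection events toggle their IsHighlighted parameter, with a leftover debug print on deselect.
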(event `self.ReceiveBeginPlay`
  (bind _niagara (`self.Niagara`))
  (bind (_direction _towergrowth _opacity) (`Timeline|Timeline_0`)
    (:`Update`
      (`NiagaraComponent.SetVariableFloat` _niagara "Progress" _towergrowth)
      (`NiagaraComponent.SetVariableFloat` _niagara "Opacity" _opacity))))

(event `self.ReceiveTick`
  (params (DeltaSeconds :type "Float (single-precision)"))
  (bind _scene (`self.Scene`))
  (bind (_returnvalue_roll _returnvalue_pitch _returnvalue_yaw) (`KismetMathLibrary.BreakRotator` (`SceneComponent.K2_GetComponentRotation` _scene)))
  (`SceneComponent.K2_SetWorldRotation` _scene (`KismetMathLibrary.MakeRotator` 0.0 0.0 (+ (* DeltaSeconds -50.0) _returnvalue_yaw)) false false))

(event `self.OnSelectEnd`
  (`KismetSystemLibrary.PrintString` "Hello")
  (`MaterialInstanceDynamic.SetScalarParameterValue` (`self.BodyMaterialInstance`) "IsHighlighted" 0.0)
  (`MaterialInstanceDynamic.SetScalarParameterValue` (`self.CubeMaterialInstance`) "IsHighlighted" 0.0))

(event `self.OnSelectStart`
  (`MaterialInstanceDynamic.SetScalarParameterValue` (`self.BodyMaterialInstance`) "IsHighlighted" 1.0)
  (`MaterialInstanceDynamic.SetScalarParameterValue` (`self.CubeMaterialInstance`) "IsHighlighted" 1.0))

(fn `UserConstructionScript`
  (bind _returnvalue (`PrimitiveComponent.CreateDynamicMaterialInstance` (`self.StructureMesh`) 0 (`self.BodyMaterialClass`) "None"))
  (set `self.BodyMaterialInstance` _returnvalue)
  (bind _returnvalue_2 (`PrimitiveComponent.CreateDynamicMaterialInstance` (`self.TypeMesh`) 0 (`self.CubeMaterialClass`) "None"))
  (set `self.CubeMaterialInstance` _returnvalue_2))