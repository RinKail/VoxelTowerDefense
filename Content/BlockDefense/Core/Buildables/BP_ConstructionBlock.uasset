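; BP_ConstructionBlock is a coloured buildable block for Block Defense that animates its own drop into the grid when spawned.
; A timeline lowers it from above while spinning it and driving a creation glow, then triggers the game mode's tile visual pulse and completes grid placement.
; A dynamic material instance handles selection highlighting, while type changes recolour its glow parameters and swap the Niagara particle material.
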(event `self.OnTypeChanged`
  (params (Type :type "EBlockType Enum" :default "BT_None"))
  (bind _returnvalue (select `EBlockType` Type :`BT_Red` (struct :`R` 1.0 :`A` 1.0) :`BT_Green` (struct :`R` 0.251775 :`G` 1.0 :`A` 1.0) :`BT_Blue` (struct :`G` 0.736899 :`B` 0.994792 :`A` 1.0) :!type "LinearColor Structure"))
  (bind _mi (`self.MI`))
  (`MaterialInstanceDynamic.SetVectorParameterValue` _mi "Glow" _returnvalue)
  (`NiagaraComponent.SetVariableMaterial` (`self.Niagara`) "Mat" (select `EBlockType` Type :`BT_Red` "/Game/BlockDefense/Art/Enviroment/Meshes/MI_ParticleBlock_Red.MI_ParticleBlock_Red" :`BT_Green` "/Game/BlockDefense/Art/Enviroment/Meshes/MI_ParticleBlock_Green.MI_ParticleBlock_Green" :`BT_Blue` "/Game/BlockDefense/Art/Enviroment/Meshes/MI_ParticleBlock_Blue.MI_ParticleBlock_Blue" :!type "MaterialInterface Object Reference"))
  (`MaterialInstanceDynamic.SetVectorParameterValue` _mi "HighlightColour" _returnvalue)
  (`MaterialInstanceDynamic.SetVectorParameterValue` _mi "CreationGlowColour" _returnvalue))

(event `self.OnSelectEnd`
  (`MaterialInstanceDynamic.SetScalarParameterValue` (`self.MI`) "IsHighlighted" 0.0))

(event `self.OnSelectStart`
  (`MaterialInstanceDynamic.SetScalarParameterValue` (`self.MI`) "IsHighlighted" 1.0))

(event `self.ReceiveBeginPlay`
  (bind (_returnvalue_x _returnvalue_y) (`KismetMathLibrary.BreakVector` (`self.K2_GetActorLocation`)))
  (bind (_returnvalue_x_2 _returnvalue_y_2 _returnvalue_z) (`KismetMathLibrary.BreakVector` (`self.K2_GetActorLocation`)))
  (bind (_returnvalue_x_3 _returnvalue_y_3) (`KismetMathLibrary.BreakVector` (`self.K2_GetActorLocation`)))
  (bind (_returnvalue_roll _returnvalue_pitch _returnvalue_yaw) (`KismetMathLibrary.BreakRotator` (`self.K2_GetActorRotation`)))
  (bind (_cachedpos_x _cachedpos_y _cachedpos_z) (`KismetMathLibrary.BreakVector` (`self.CachedPos`)))
  ;[1 1 1] Comment
  (`|ExecutionSequence`
    (:`then_0`
      (set `self.CachedPos` (`self.K2_GetActorLocation`))
      (`MaterialInstanceDynamic.SetScalarParameterValue` (`self.MI`) "CreationGlowLerp" 1.0)
      (`self.K2_SetActorLocation` (+ (`self.K2_GetActorLocation`) (0.0 0.0 1000.0)))
      (bind _output_get (set `self.CachedRot` _returnvalue_yaw))
      (bind (_direction _alpha _rot _glowlerp) (`Timeline|Timeline_0` :!via `PlayFromStart`)
        (:`Update`
          (`self.K2_SetActorLocation` (`KismetMathLibrary.VLerp` (`KismetMathLibrary.MakeVector` _returnvalue_x _returnvalue_y (+ _cachedpos_z 1000.0)) (`KismetMathLibrary.MakeVector` _cachedpos_x _cachedpos_y _cachedpos_z) _alpha))
          (`self.K2_SetActorRotation` (`KismetMathLibrary.MakeRotator` _returnvalue_roll _returnvalue_pitch (+ _rot _output_get)))
          (`MaterialInstanceDynamic.SetScalarParameterValue` (`self.MI`) "CreationGlowLerp" _glowlerp))
        (:`Finished`
          (`MaterialInstanceDynamic.SetVectorParameterValue` (`self.MI`) "HighlightColour" (struct :`R` 0.8125 :`G` 0.26366 :`A` 1.0))
          (`BlockDefenseGameMode.TriggerTileUpdateVisualEvent` (cast `BlockDefenseGameMode` (`GameplayStatics.GetGameMode`) :!pure true) (`KismetMathLibrary.MakeVector` _returnvalue_x_3 _returnvalue_y_3) (+ (/ _returnvalue_z 200.0) 0.1))
          (`Map_ConstructionGrid.CompletePlacement` (`self.GetGrid`) self))))))

(fn `UserConstructionScript`
  (bind _returnvalue (`PrimitiveComponent.CreateDynamicMaterialInstance` (`self.MeshComponent`) 0 "/Game/BlockDefense/Art/Enviroment/Meshes/MI_ConstructionBlock.MI_ConstructionBlock" "None"))
  (set `self.MI` _returnvalue))