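; Base map tile for Block Defense that randomises its height scale and quarter-turn yaw on construction and animates itself through timelines.
; Creation drops the tile from above with rotation, Niagara and a material glow.
; Game start settles tiles from StartHeight, delayed by distance from the protection target, while nearby tile changes trigger a distance-delayed, intensity-scaled Z ripple.
; A dynamic material also shows green or red highlights based on TransformConditionsMet.
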(event `self.OnCreation`
  (bind (_returnvalue_x _returnvalue_y) (`KismetMathLibrary.BreakVector` (`self.K2_GetActorLocation`)))
  (bind (_returnvalue_roll _returnvalue_pitch _returnvalue_yaw) (`KismetMathLibrary.BreakRotator` (`self.K2_GetActorRotation`)))
  ;[1 1 1] Comment
  (`ActorComponent.Activate` (`self.Niagara`) true)
  (`MaterialInstanceDynamic.SetScalarParameterValue` (`self.StoredResource`) "CreationGlowLerp" 1.0)
  (`self.K2_SetActorLocation` (+ (`self.K2_GetActorLocation`) (0.0 0.0 1000.0)))
  (bind _output_get (set `self.CachedRot` _returnvalue_yaw))
  (bind (_direction _alpha _rot _glowlerp) (`Timeline|Timeline_Creation` :!via `PlayFromStart`)
    (:`Update`
      (`self.K2_SetActorLocation` (`KismetMathLibrary.VLerp` (`KismetMathLibrary.MakeVector` _returnvalue_x _returnvalue_y 1000.0) (`KismetMathLibrary.MakeVector` _returnvalue_x _returnvalue_y) _alpha))
      (`self.K2_SetActorRotation` (`KismetMathLibrary.MakeRotator` _returnvalue_roll _returnvalue_pitch (+ _rot _output_get)))
      (`MaterialInstanceDynamic.SetScalarParameterValue` (`self.StoredResource`) "CreationGlowLerp" _glowlerp))))

(event `self.OnGameStart`
  (bind (_returnvalue_x _returnvalue_y) (`KismetMathLibrary.BreakVector` (`self.K2_GetActorLocation`)))
  (bind _startheight (`self.StartHeight`))
  ;[1 1 1] Comment
  (bind _outactors (`GameplayStatics.GetAllActorsOfClass` "/Script/BlockDefense.Map_ProtectionTarget"))
  (`self.K2_SetActorLocation` (+ (`self.K2_GetActorLocation`) (`KismetMathLibrary.MakeVector` 0.0 0.0 _startheight)))
  (bind (_returnvalue_x_2 _returnvalue_y_2) (`KismetMathLibrary.BreakVector` (`self.K2_GetActorLocation` (`|GetArrayItem` _outactors))))
  (`KismetSystemLibrary.Delay` (/ (`KismetMathLibrary.Vector_Distance` (`self.K2_GetActorLocation`) (`KismetMathLibrary.MakeVector` _returnvalue_x_2 _returnvalue_y_2 _startheight)) 1250.0))
  (bind (_direction _alpha) (`Timeline|Timeline_GameStart`)
    (:`Update`
      (`self.K2_SetActorLocation` (`KismetMathLibrary.VLerp` (`KismetMathLibrary.MakeVector` _returnvalue_x _returnvalue_y (`self.StartHeight`)) (`KismetMathLibrary.MakeVector` _returnvalue_x _returnvalue_y) _alpha)))))

(event `self.OnTileChanged`
  (params (TilePosition :type "Vector Structure") (Intensity :type "Float (single-precision)"))
  (bind (_returnvalue_x _returnvalue_y) (`KismetMathLibrary.BreakVector` (`self.K2_GetActorLocation`)))
  (bind _returnvalue (/ (`KismetMathLibrary.Vector_Distance` (`self.K2_GetActorLocation`) TilePosition) (* Intensity 1250.0)))
  (if (<= _returnvalue 1.5)
    (`KismetSystemLibrary.Delay` (`KismetMathLibrary.SelectFloat` (+ _returnvalue 0.1) (- _returnvalue 0.1) (<= Intensity 1.0)))
    (bind (_direction _alpha) (`Timeline|Timeline_TileUpdate` :!via `PlayFromStart`)
      (:`Update`
        (`self.K2_SetActorLocation` (`KismetMathLibrary.VLerp` (`KismetMathLibrary.MakeVector` _returnvalue_x _returnvalue_y) (`KismetMathLibrary.MakeVector` _returnvalue_x _returnvalue_y (* Intensity 75.0)) _alpha))))))

(event `self.ReceiveBeginPlay`
  (bind _returnvalue (`PrimitiveComponent.CreateDynamicMaterialInstance` (`self.MeshComponent`) 0 "/Game/BlockDefense/Art/Enviroment/Meshes/MI_Tile_Resource.MI_Tile_Resource" "None"))
  (set `self.StoredResource` _returnvalue))

(event `self.OnHighlightEnd`
  (`MaterialInstanceDynamic.SetScalarParameterValue` (`self.StoredResource`) "IsHighlighted" 0.0))

(event `self.OnHighlightStart`
  (`MaterialInstanceDynamic.SetVectorParameterValue` (`self.StoredResource`) "HighlightColour" (`KismetMathLibrary.SelectColor` (struct :`G` 1.0 :`B` 0.0375 :`A` 1.0) (struct :`R` 0.8125 :`G` 0.078107 :`A` 1.0) (`self.bTransformConditionsMet`)))
  (`MaterialInstanceDynamic.SetScalarParameterValue` (`self.StoredResource`) "IsHighlighted" 1.0))

(fn `UserConstructionScript`
  (`self.SetActorScale3D` (`KismetMathLibrary.MakeVector` 1.0 1.0 (`KismetMathLibrary.RandomFloatInRange` 1.0 (`self.TileHeightVariance`))))
  (`self.K2_SetActorRotation` (`KismetMathLibrary.MakeRotator` 0.0 0.0 (select `int` (`KismetMathLibrary.RandomIntegerInRange` 0 3) :`0` 0.0 :`1` 90.0 :`2` 180.0 :`3` 270.0 :!type "Float (single-precision)"))))