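; Passage tile for the Block Defense map, with randomized height scale and 90-degree yaw set at construction.
; On creation it jumps up and eases down by timeline after a short delay.
; At game start it does the same from StartHeight, delayed by distance to the first Map_ProtectionTarget so the drop-in is staggered.
; Highlight events toggle a scalar on a dynamic material created at BeginPlay.
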(event `self.OnCreation`
  (bind (_returnvalue_x _returnvalue_y) (`KismetMathLibrary.BreakVector` (`self.K2_GetActorLocation`)))
  ;[1 1 1] Comment
  (`self.K2_SetActorLocation` (+ (`self.K2_GetActorLocation`) (0.0 0.0 1000.0)))
  (`KismetSystemLibrary.Delay` 0.5)
  (bind (_direction _alpha) (`Timeline|Timeline_1` :!via `PlayFromStart`)
    (:`Update`
      (`self.K2_SetActorLocation` (`KismetMathLibrary.VLerp` (`KismetMathLibrary.MakeVector` _returnvalue_x _returnvalue_y 1000.0) (`KismetMathLibrary.MakeVector` _returnvalue_x _returnvalue_y) _alpha)))))

(event `self.OnGameStart`
  (bind (_returnvalue_x _returnvalue_y) (`KismetMathLibrary.BreakVector` (`self.K2_GetActorLocation`)))
  (bind _startheight (`self.StartHeight`))
  (bind _outactors (`GameplayStatics.GetAllActorsOfClass` "/Script/BlockDefense.Map_ProtectionTarget"))
  ;[1 1 1] Comment
  (`self.K2_SetActorLocation` (+ (`self.K2_GetActorLocation`) (`KismetMathLibrary.MakeVector` 0.0 0.0 _startheight)))
  (bind (_returnvalue_x_2 _returnvalue_y_2) (`KismetMathLibrary.BreakVector` (`self.K2_GetActorLocation` (`|GetArrayItem` _outactors))))
  (`KismetSystemLibrary.Delay` (/ (`KismetMathLibrary.Vector_Distance` (`self.K2_GetActorLocation`) (`KismetMathLibrary.MakeVector` _returnvalue_x_2 _returnvalue_y_2 _startheight)) 750.0))
  (bind (_direction _alpha) (`Timeline|Timeline_0`)
    (:`Update`
      (`self.K2_SetActorLocation` (`KismetMathLibrary.VLerp` (`KismetMathLibrary.MakeVector` _returnvalue_x _returnvalue_y (`self.StartHeight`)) (`KismetMathLibrary.MakeVector` _returnvalue_x _returnvalue_y) _alpha)))))

(event `self.ReceiveBeginPlay`
  (bind _returnvalue (`PrimitiveComponent.CreateDynamicMaterialInstance` (`self.MeshComponent`) 0 "/Game/BlockDefense/Art/Enviroment/Meshes/MI_Tile_Resource.MI_Tile_Resource" "None"))
  (set `self.StoredResource` _returnvalue))

(event `self.OnHighlightEnd`
  (`MaterialInstanceDynamic.SetScalarParameterValue` (`self.StoredResource`) "IsHighlighted" 0.0))

(event `self.OnHighlightStart`
  (`MaterialInstanceDynamic.SetScalarParameterValue` (`self.StoredResource`) "IsHighlighted" 1.0))

(fn `UserConstructionScript`
  (`self.SetActorScale3D` (`KismetMathLibrary.MakeVector` 1.0 1.0 (`KismetMathLibrary.RandomFloatInRange` 1.0 (`self.TileHeightVariance`))))
  (`self.K2_SetActorRotation` (`KismetMathLibrary.MakeRotator` 0.0 0.0 (select `int` (`KismetMathLibrary.RandomIntegerInRange` 0 3) :`0` 0.0 :`1` 90.0 :`2` 180.0 :`3` 270.0 :!type "Float (single-precision)"))))