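; BP_PlayerView is the player's camera rig in BlockDefense, handling view zoom, rotation and a game speed toggle.
; On BeginPlay, a timeline lerps the spring arm length from far to near as an intro zoom.
; The Zoom axis adjusts arm length within clamped limits, while RotateCamera yaws the whole actor.
; The T key flip-flops global time dilation between fast-forward and normal speed.
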(event `self.ReceiveBeginPlay`
  (set `SpringArmComponent.TargetArmLength` 1500.0 (`self.SpringArm`))
  (bind (_direction _newtrack_0) (`Timeline|Timeline_0`)
    (:`Update`
      (set `SpringArmComponent.TargetArmLength` (`KismetMathLibrary.Lerp` 1800.0 300.0 _newtrack_0) (`self.SpringArm`)))))

(event `InputAxis|Zoom`
  (params (AxisValue :type "Float (single-precision)"))
  (bind _springarm (`self.SpringArm`))
  (set `SpringArmComponent.TargetArmLength` (`KismetMathLibrary.FClamp` (+ (* (* AxisValue (`self.ZoomMultiplier`)) -1.0) (`SpringArmComponent.TargetArmLength` _springarm)) 300.0 1000.0) _springarm))

(event `InputAxis|RotateCamera`
  (params (AxisValue :type "Float (single-precision)"))
  (bind (_returnvalue_roll _returnvalue_pitch _returnvalue_yaw) (`KismetMathLibrary.BreakRotator` (`self.K2_GetActorRotation`)))
  (`self.K2_SetActorRotation` (`KismetMathLibrary.MakeRotator` 0.0 0.0 (+ (* AxisValue (`self.RotationMultiplier`)) _returnvalue_yaw))))

(event `Key|T`
  (params (Key :type "Key Structure"))
  (:`Pressed`
    (`/Engine/EditorBlueprintResources/StandardMacros.FlipFlop`
      (:`A`
        (`GameplayStatics.SetGlobalTimeDilation` 3.0))
      (:`B`
        (`GameplayStatics.SetGlobalTimeDilation` 1.0)))))

(fn `UserConstructionScript`)