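; Tutorial game mode for Block Defense that drives the HUD, staged tutorial popups and end screens.
; On BeginPlay it shows the wave counter HUD, then the tower-building popup after a short delay.
; Wave-end events switch on the current wave to show structure-building and damage-type popups, then a level-complete screen after the fourth wave.
; Game over brings up the game over widget.
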(event `self.ReceiveBeginPlay`
  (bind _returnvalue (`|CreateWidget` "/Game/BlockDefense/Core/UI/HUD/W_HUD_WaveCounter.W_HUD_WaveCounter_C" null self))
  (`UserWidget.AddToViewport` _returnvalue 0)
  (`KismetSystemLibrary.Delay` 4.0)
  (bind _returnvalue_2 (`|CreateWidget` "/Game/BlockDefense/Core/UI/Tutorial/W_TutorialPopup.W_TutorialPopup_C" null "TowerBuilding"))
  (`UserWidget.AddToViewport` _returnvalue_2 0))

(event `self.OnGameOver`
  (bind _returnvalue (`|CreateWidget` "/Game/BlockDefense/Core/UI/GameOverMenu/W_GameOver.W_GameOver_C"))
  (`UserWidget.AddToViewport` _returnvalue 0))

(event `self.OnWaveEnd`
  (switch `int` (`self.GetCurrentWave`)
    (:`1`
      (bind _returnvalue (`|CreateWidget` "/Game/BlockDefense/Core/UI/Tutorial/W_TutorialPopup.W_TutorialPopup_C" null "StructureBuilding"))
      (`UserWidget.AddToViewport` _returnvalue 0))
    (:`2`
      (bind _returnvalue_2 (`|CreateWidget` "/Game/BlockDefense/Core/UI/Tutorial/W_TutorialPopup.W_TutorialPopup_C" null "DamageTypes"))
      (`UserWidget.AddToViewport` _returnvalue_2 0))
    (:`4`
      (bind _returnvalue_3 (`|CreateWidget` "/Game/BlockDefense/Core/UI/GameOverMenu/W_LevelComplete.W_LevelComplete_C"))
      (`UserWidget.AddToViewport` _returnvalue_3 0))))

(fn `UserConstructionScript`)