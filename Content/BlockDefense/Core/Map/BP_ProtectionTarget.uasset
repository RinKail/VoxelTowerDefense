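; BP_ProtectionTarget is the core actor to protect in Block Defense, shown as a spinning block with a HUD health bar.
; On BeginPlay it creates the health bar widget, passing itself as the core reference.
; When damaged, it has the game mode trigger a tile visual update at its location, scaled by damage.
; Tick spins the Scene component in pitch and BlockFrame in yaw, zeroing their other axes.
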(event `self.ReceiveBeginPlay`
  (bind _returnvalue (`|CreateWidget` "/Game/BlockDefense/Core/UI/HUD/W_HUD_HealthBar.W_HUD_HealthBar_C" null self))
  (`UserWidget.AddToViewport` _returnvalue 0))

(event `self.OnDamageTaken`
  (params (DamageTaken :type Integer))
  (`BlockDefenseGameMode.TriggerTileUpdateVisualEvent` (cast `BlockDefenseGameMode` (`GameplayStatics.GetGameMode`) :!pure true) (`self.K2_GetActorLocation`) (`KismetMathLibrary.Conv_IntToDouble` DamageTaken)))

(event `self.ReceiveTick`
  (params (DeltaSeconds :type "Float (single-precision)"))
  (bind _blockframe (`self.BlockFrame`))
  (bind _scene (`self.Scene`))
  (bind (_returnvalue_roll _returnvalue_pitch _returnvalue_yaw) (`KismetMathLibrary.BreakRotator` (`SceneComponent.K2_GetComponentRotation` _blockframe)))
  (bind (_returnvalue_roll_2 _returnvalue_pitch_2 _returnvalue_yaw_2) (`KismetMathLibrary.BreakRotator` (`SceneComponent.K2_GetComponentRotation` _scene)))
  (`SceneComponent.K2_SetWorldRotation` _scene (`KismetMathLibrary.MakeRotator` 0.0 (+ (* DeltaSeconds -50.0) _returnvalue_pitch_2)) false false)
  (`SceneComponent.K2_SetWorldRotation` _blockframe (`KismetMathLibrary.MakeRotator` 0.0 0.0 (+ (* DeltaSeconds -50.0) _returnvalue_yaw)) false false))

(fn `UserConstructionScript`)